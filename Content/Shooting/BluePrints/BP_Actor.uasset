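; BP_Actor is an actor that times how long a BP_ShootingCharacter stays inside its Cube component.
; The Cube's begin and end overlap events set a single IsOverlap flag, only on the server through authority checks.
; Tick adds delta time to TotalSec while the flag is set and resets it to zero otherwise.
; Nothing in the graph acts on the accumulated time.
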(event OnComponentBeginOverlap(Cube)
  (params (OverlappedComponent :type Primitive%20Component%20Object%20Reference) (OtherActor :type Actor%20Object%20Reference) (OtherComp :type Primitive%20Component%20Object%20Reference) (OtherBodyIndex :type Integer) (bFromSweep :type Boolean) (SweepResult :type Hit%20Result%20Structure%20%28by%20ref%29))
  ;[0.15 0.15 0.15 0.5] 서버만!!
  (Networking|SwitchHasAuthority
    (:Authority
      (Utilities|Casting|CastToBP_ShootingCharacter OtherActor)
      (Variables|Default|SetIsOverlap true))))

(event OnComponentEndOverlap(Cube)
  (params (OverlappedComponent :type Primitive%20Component%20Object%20Reference) (OtherActor :type Actor%20Object%20Reference) (OtherComp :type Primitive%20Component%20Object%20Reference) (OtherBodyIndex :type Integer))
  (Networking|SwitchHasAuthority
    (:Authority
      (Utilities|Casting|CastToBP_ShootingCharacter OtherActor)
      (Variables|Default|SetIsOverlap false))))

(event EventTick
  (params (DeltaSeconds :type Float%20%28single-precision%29))
  (if (Variables|Default|GetIsOverlap)
    (Variables|Default|SetTotalSec (+ DeltaSeconds (Variables|Default|GetTotalSec)))
    (else
      (Variables|Default|SetTotalSec 0.0))))

(fn ConstructionScript)