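; Shooting game HUD Blueprint that displays the local player's current and max HP.
; On BeginPlay it creates BP_ShootingHudWidget, adds it to the viewport and binds to the UpdateHP dispatcher on BP_ShootingPlayerState.
; Binding also pushes the initial HP values to the widget through EventUpdateHP.
; If the player state cast fails, a short timer retries binding to cover late PlayerState creation.
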(event EventBeginPlay
  (bind _returnvalue (UserInterface|CreateWidget "/Game/Shooting/widgets/BP_ShootingHudWidget.BP_ShootingHudWidget_C"))
  (bind _output_get (Variables|Default|SetHudWidget _returnvalue))
  (UserInterface|Viewport|AddtoViewport (Variables|Default|GetHudWidget) 0)
  (CallFunction|BindPlayerState))

(fn ConstructionScript)

(fn UpdateHP
  (params (CurHP :type Float%20%28double-precision%29) (MaxHP :type Float%20%28double-precision%29))
  (Default|UpdateHP (Variables|Default|GetHudWidget) CurHP MaxHP))

(fn BindPlayerState
  (bind _asbp_shooting_player_state (Utilities|Casting|CastToBP_ShootingPlayerState (Variables|/Script/Engine.Controller|GetPlayerState (Game|GetPlayerController 0)))
    (:then
      (EventDispatchers|BindEventtoEventDispatcherUpdateHP _asbp_shooting_player_state (EventDispatchers|CreateEvent :!event EventUpdateHP))
      (CallFunction|EventUpdateHP (Variables|/Game/Shooting/GameMOd/BP_ShootingPlayerState.BP_ShootingPlayerState_C|GetCurHP _asbp_shooting_player_state) (Variables|/Game/Shooting/GameMOd/BP_ShootingPlayerState.BP_ShootingPlayerState_C|GetMaxHP _asbp_shooting_player_state)))
    (:CastFailed
      ;[0.15 0.15 0.15 0.5] playerstate함수가 BindPlayerState보다 늦게 생성될 확률도 있기에, 다시 BindPlayerState를 실행시킨다
      (Utilities|Time|SetTimerbyFunctionName 0 "BindPlayerState" 0.1))))

(fn EventUpdateHP
  (params (CurHP :type Float%20%28double-precision%29) (MaxHP :type Float%20%28double-precision%29))
  (Default|UpdateHP (Variables|Default|GetHudWidget) CurHP MaxHP))