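; Burst-fire weapon Blueprint that fires a three-shot burst on a trigger press by extending its parent's Dotrigger.
; EventTrigger resets ShootCount and starts a short looping timer on Dotrigger.
; Dotrigger calls the parent implementation, counts the shot and clears the timer after the third.
; The guard against restarting checks TimerExists with an empty function name, so it does not reference the Dotrigger timer.
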(event EventBeginPlay)

(event Collision|EventActorBeginOverlap
  (params (OtherActor :type Actor%20Object%20Reference)))

(event EventTick
  (params (DeltaSeconds :type Float%20%28single-precision%29)))

(fn ConstructionScript
  (|CallParentFunction))

(fn EventTrigger
  (params (IsPress :type Boolean))
  (if IsPress
    (if (not (Class|KismetSystemLibrary|TimerExists))
      (Variables|Default|SetShootCount 0)
      (Utilities|Time|SetTimerbyFunctionName 0 "Dotrigger" 0.1 true)
      (return true))))

(fn Dotrigger
  (|CallParentFunction)
  (bind _output_get (Variables|Default|SetShootCount (+ (Variables|Default|GetShootCount) 1)))
  (if (>= _output_get 3)
    (Utilities|Time|ClearTimerbyFunctionName 0 "Dotrigger")))