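; Actor component that gives its owner an on-screen name tag showing name and HP.
; On BeginPlay it creates a NameTagWidget, passes itself in as the widget's NameTagComponent and adds it to the viewport, then removes it on EndPlay.
; SetName and SetHp forward name and current/max HP straight to that widget.
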(event EventBeginPlay
  (bind _returnvalue (UserInterface|CreateWidget "/Game/Shooting/Nametag/NameTagWidget.NameTagWidget_C" 0 self))
  (bind _output_get (Variables|Default|SetNameTag _returnvalue))
  (UserInterface|Viewport|AddtoViewport _output_get 0))

(event EventEndPlay
  (params (EndPlayReason :type EEndPlayReason%20Enum :default "Destroyed"))
  (Widget|RemovefromParent (Variables|Default|GetNameTag)))

(fn SetName
  (params (Name :type String))
  (Default|SetName (Variables|Default|GetNameTag) Name))

(fn SetHp
  (params (CurHp :type Float%20%28double-precision%29) (MaxHp :type Float%20%28double-precision%29))
  (Default|SetHp (Variables|Default|GetNameTag) CurHp MaxHp))